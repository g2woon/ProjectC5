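; BP_MoveRect is a practice Blueprint that moves its MoveRect component around a square path in the relative XZ plane.
; While IsPlay is true, Tick steps Location by Speed per frame, without delta-time scaling, and applies it as relative location.
; The EnSwitch enum picks the direction and advances when Location crosses the square's bounds.
; Unconnected leftovers hold a frame-count version and String, Name and Int switch experiments.
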(event EventTick
  (params (DeltaSeconds :type Float%20%28single-precision%29))
  (if (Variables|Default|GetIsPlay)
    ;[0.15 0.15 0.15 0.5] 사각이동 Case 2 - Count 안씀
    (switch Utilities|FlowControl|Switch|SwitchonEN_MoveType (Variables|Default|GetEnSwitch)
      (:NewEnumerator0
        ;;[0.15 0.15 0.15 0.5] MoveRight
        (bind _output_get (Variables|Default|SetLocation (+ (Variables|Default|GetLocation) (Math|Vector|MakeVector (* (Variables|Default|GetSpeed) 1.0) 0.0 0.0))))
        (Transformation|SetRelativeLocation (Variables|Default|GetMoveRect) _output_get false false)
        (if (> (.x (Variables|Default|GetLocation)) 5e+02)
          (Variables|Default|SetEnSwitch "NewEnumerator1")))
      (:NewEnumerator1
        ;;[0.15 0.15 0.15 0.5] MoveUp
        (bind _output_get_2 (Variables|Default|SetLocation (+ (Variables|Default|GetLocation) (Math|Vector|MakeVector 0.0 0.0 (* (Variables|Default|GetSpeed) 1.0)))))
        (Transformation|SetRelativeLocation (Variables|Default|GetMoveRect) _output_get_2 false false)
        (if (> (.z (Variables|Default|GetLocation)) 5e+02)
          (Variables|Default|SetEnSwitch "NewEnumerator2")))
      (:NewEnumerator2
        ;;[0.15 0.15 0.15 0.5] MoveLeft
        (bind _output_get_3 (Variables|Default|SetLocation (+ (Variables|Default|GetLocation) (Math|Vector|MakeVector (* (Variables|Default|GetSpeed) -1.0) 0.0 0.0))))
        (Transformation|SetRelativeLocation (Variables|Default|GetMoveRect) _output_get_3 false false)
        (if (< (.x (Variables|Default|GetLocation)) 0.0)
          (Variables|Default|SetEnSwitch "NewEnumerator3")))
      (:NewEnumerator3
        ;;[0.15 0.15 0.15 0.5] MoveDown
        (bind _output_get_4 (Variables|Default|SetLocation (+ (Variables|Default|GetLocation) (Math|Vector|MakeVector 0.0 0.0 (* (Variables|Default|GetSpeed) -1.0)))))
        (Transformation|SetRelativeLocation (Variables|Default|GetMoveRect) _output_get_4 false false)
        (if (< (.z (Variables|Default|GetLocation)) 0.0)
          (Variables|Default|SetEnSwitch "NewEnumerator0"))))))

(fn ConstructionScript)