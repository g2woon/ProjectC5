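; BP_Spawner is an actor that spawns a batch of ten actors at random points inside its Box component.
; The DoSpawn event loops on a Count variable, picking each location within the box's scaled extent around the actor's location and reusing the spawner's rotation.
; After the loop it resets Count so the event can run again, then prints a completion message.
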(event Custom|DoSpawn
  (bind _returnvalue (Transformation|GetActorLocation))
  (bind _box (Variables|Default|GetBox))
  (bind _returnvalue_2 (Components|Box|GetScaledBoxExtent _box))
  (bind _returnvalue_3 (Math|Random|RandomPointinBoundingBox _returnvalue _returnvalue_2))
  (while (< (Variables|Default|GetCount) 10)
    (Development|PrintString (Utilities|String|Append "index : " (Utilities|String|ToString(Integer) (Variables|Default|GetCount))) true true "(R=0.000000,G=0.660000,B=1.000000,A=1.000000)" 6e+01)
    (Variables|Default|SetCount (+ (Variables|Default|GetCount) 1))
    (Development|PrintString (Utilities|String|ToString(Vector) _returnvalue_3))
    (Game|SpawnActorfromClass "/Game/HelloUnreal/BP_Ball.BP_Ball_C" (Math|Transform|MakeTransform _returnvalue_3 (Transformation|GetActorRotation) "1.000000,1.000000,1.000000") "Undefined" "MultiplyWithRoot" 0 0))
  (Variables|Default|SetCount 0)
  (Development|PrintString "Complete" true true "(R=0.000000,G=0.660000,B=1.000000,A=1.000000)" 6e+01))

(fn ConstructionScript)