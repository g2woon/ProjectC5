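; BP_Switch is an overlap switch that runs linked moving actors while something overlaps its Cube component.
; Begin overlap sets IsPlay on MoveActor, MoveRect and MoveStair, and end overlap clears it, each behind a validity check.
; Each begin overlap also calls DoSpawn on Spawner until SpawnCount hits its cap, with no validity check.
; The debug prints are disabled and the Spawner DestroyActor call is unwired.
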(event OnComponentBeginOverlap(Cube)
  (params (OverlappedComponent :type Primitive%20Component%20Object%20Reference) (OtherActor :type Actor%20Object%20Reference) (OtherComp :type Primitive%20Component%20Object%20Reference) (OtherBodyIndex :type Integer) (bFromSweep :type Boolean) (SweepResult :type Hit%20Result%20Structure%20%28by%20ref%29))
  (bind _moveactor (Variables|Default|GetMoveActor))
  (bind _moverect (Variables|Default|GetMoveRect))
  (bind _movestair (Variables|Default|GetMoveStair))
  (Development|PrintString (Utilities|String|Append "Begin Overlap  ||  " "Overlapped Component : " (Utilities|GetDisplayName OverlappedComponent) ", Other Actor : " (Utilities|GetDisplayName OtherActor) ", Other Comp : " (Utilities|GetDisplayName OtherComp)) true true "(R=0.000000,G=0.660000,B=1.000000,A=1.000000)" 1.0)
  (Utilities|FlowControl|Sequence
    (:then_0
      (Utilities|IsValid _moveactor
        (:Is%20Valid
          (Variables|/Game/HelloUnreal/BP_MoveActor.BP_MoveActor_C|SetIsPlay _moveactor true))
        (:Is%20Not%20Valid
          (Development|PrintString "MoveActor is Nullptr!!" true true "(R=1.000000,G=0.000000,B=0.000000,A=1.000000)"))))
    (:then_1
      (Utilities|IsValid _moverect
        (:Is%20Valid
          (Variables|/Game/HelloUnreal/BP_MoveRect.BP_MoveRect_C|SetIsPlay _moverect true))
        (:Is%20Not%20Valid
          (Development|PrintString "MoveRect is Nullptr!!" true true "(R=1.000000,G=0.000000,B=0.000000,A=1.000000)"))))
    (:then_2
      (Utilities|IsValid _movestair
        (:Is%20Valid
          (Variables|/Game/HelloUnreal/BP_MoveStair.BP_MoveStair_C|SetIsPlay _movestair true))
        (:Is%20Not%20Valid
          (Development|PrintString "MoveStair is Nullptr!!" true true "(R=1.000000,G=0.000000,B=0.000000,A=1.000000)"))))
    (:then_3
      (if (< (Variables|Default|GetSpawnCount) 20)
        (Variables|Default|SetSpawnCount (+ (Variables|Default|GetSpawnCount) 1))
        (Default|DoSpawn (Variables|Default|GetSpawner))))))

(event OnComponentEndOverlap(Cube)
  (params (OverlappedComponent :type Primitive%20Component%20Object%20Reference) (OtherActor :type Actor%20Object%20Reference) (OtherComp :type Primitive%20Component%20Object%20Reference) (OtherBodyIndex :type Integer))
  (bind _moverect (Variables|Default|GetMoveRect))
  (bind _movestair (Variables|Default|GetMoveStair))
  (bind _moveactor (Variables|Default|GetMoveActor))
  (Development|PrintString (Utilities|String|Append "End Overlap  ||  " "Overlapped Component : " (Utilities|GetDisplayName OverlappedComponent) ", Other Actor : " (Utilities|GetDisplayName OtherActor) ", Other Comp : " (Utilities|GetDisplayName OtherComp)) true true "(R=0.000000,G=0.660000,B=1.000000,A=1.000000)" 1.0)
  (Utilities|FlowControl|Sequence
    (:then_0
      (Utilities|IsValid _moveactor
        (:Is%20Valid
          (Variables|/Game/HelloUnreal/BP_MoveActor.BP_MoveActor_C|SetIsPlay _moveactor false))
        (:Is%20Not%20Valid
          (Development|PrintString "MoveActor is Nullptr!!" true true "(R=1.000000,G=0.000000,B=0.000000,A=1.000000)"))))
    (:then_1
      (Utilities|IsValid _moverect
        (:Is%20Valid
          (Variables|/Game/HelloUnreal/BP_MoveRect.BP_MoveRect_C|SetIsPlay _moverect false))
        (:Is%20Not%20Valid
          (Development|PrintString "MoveRect is Nullptr!!" true true "(R=1.000000,G=0.000000,B=0.000000,A=1.000000)"))))
    (:then_2
      (Utilities|IsValid _movestair
        (:Is%20Valid
          (Variables|/Game/HelloUnreal/BP_MoveStair.BP_MoveStair_C|SetIsPlay _movestair false))
        (:Is%20Not%20Valid
          (Development|PrintString "MoveStair is Nullptr!!" true true "(R=1.000000,G=0.000000,B=0.000000,A=1.000000)"))))))

(fn ConstructionScript)